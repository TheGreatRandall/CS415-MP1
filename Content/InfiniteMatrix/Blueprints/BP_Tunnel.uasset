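; BP_Tunnel is an endless-tunnel segment with a spinning holed wall, spawning an enemy and possibly a health pickup at randomized construction-time positions.
; Passing the trigger adds score; hitting the wall costs health and score, shakes the camera and shows restart at zero health.
; Either outcome requests another tunnel from TunnelSpawner, then destroys the segment and its spawned actors.
; RandomizeWall provides random mesh and roll but is not called here.
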(event `self.ReceiveBeginPlay`
  (`|ExecutionSequence`
    (:`then_0`
      (if (`KismetMathLibrary.RandomBoolWithWeight` 0.6)
        (bind _returnvalue (`|SpawnActorFromClass` "/Game/InfiniteMatrix/Blueprints/BP_Health.BP_Health_C" (`KismetMathLibrary.MakeTransform` (`SceneComponent.K2_GetComponentLocation` (`self.Health`)) (struct) (5.0 5.0 5.0)) "Undefined" "OverrideRootScale" null null))
        (set `self.spawnhealth` _returnvalue)))
    (:`then_1`
      (bind _returnvalue_2 (`|SpawnActorFromClass` "/Game/InfiniteMatrix/Blueprints/BP_enemy.BP_enemy_C" (`KismetMathLibrary.MakeTransform` (`SceneComponent.K2_GetComponentLocation` (`self.Eenemy`)) (struct :`Yaw` 90.0) (0.5 0.5 0.5)) "Undefined" "OverrideRootScale" null null))
      (set `self.spawnenemy` _returnvalue_2))
    (:`then_2`
      (bind _asbp_player (cast `/Game/InfiniteMatrix/Blueprints/BP_Player` (`GameplayStatics.GetPlayerPawn` 0)))
      (set `self.As BP Player` _asbp_player))))

(event `self.ReceiveTick`
  (params (DeltaSeconds :type "Float (single-precision)"))
  (`SceneComponent.K2_AddLocalRotation` (`self.WallMesh`) (`KismetMathLibrary.MakeRotator` (* DeltaSeconds (`self.RotateSpeed`))) false false))

(event `self.TriggerZone.OnComponentBeginOverlap`
  (params (OverlappedComponent :type "PrimitiveComponent Object Reference") (OtherActor :type "Actor Object Reference") (OtherComp :type "PrimitiveComponent Object Reference") (OtherBodyIndex :type Integer) (bFromSweep :type Boolean) (SweepResult :type "HitResult Structure (by ref)"))
  (cast `/Game/InfiniteMatrix/Blueprints/BP_Player` OtherActor)
  (`/Game/InfiniteMatrix/Blueprints/BP_TunnelSpawner.SpawnTunnelAtSpawnPoint` (`self.TunnelSpawner`))
  (`/Game/InfiniteMatrix/Blueprints/BP_Player.AddScore` (`self.As BP Player`) 10 true)
  (`self.clear`)
  (`self.K2_DestroyActor`))

(event `self.WallMesh.OnComponentHit`
  (params (HitComponent :type "PrimitiveComponent Object Reference") (OtherActor :type "Actor Object Reference") (OtherComp :type "PrimitiveComponent Object Reference") (NormalImpulse :type "Vector Structure") (Hit :type "HitResult Structure (by ref)"))
  (bind _asbp_player (cast `/Game/InfiniteMatrix/Blueprints/BP_Player` OtherActor))
  (bind _output_get (set `/Game/InfiniteMatrix/Blueprints/BP_Player.Health` (`KismetMathLibrary.FClamp` (- (`/Game/InfiniteMatrix/Blueprints/BP_Player.Health` _asbp_player) 20.0) 0.0 100.0) _asbp_player))
  (`KismetSystemLibrary.PrintString` (`KismetStringLibrary.Conv_DoubleToString` _output_get))
  (`/Game/InfiniteMatrix/Blueprints/BP_TunnelSpawner.SpawnTunnelAtSpawnPoint` (`self.TunnelSpawner`))
  (`self.K2_DestroyActor`)
  (`self.clear`)
  (`/Game/InfiniteMatrix/Blueprints/BP_Player.AddScore` _asbp_player 5 false)
  (`CameraShakeSourceComponent.StartCameraShake` :`self` (`/Game/InfiniteMatrix/Blueprints/BP_Player.CameraShakeSource` _asbp_player) :`InCameraShake` "/Game/InfiniteMatrix/Blueprints/NewBlueprint.NewBlueprint_C" :`Scale` 5.0)
  (if (== (`/Game/InfiniteMatrix/Blueprints/BP_Player.Health` _asbp_player) 0.0)
    (`/Game/InfiniteMatrix/Blueprints/BP_Player.DisplayRestart` _asbp_player)))

(fn `clear`
  (bind _spawnenemy (`self.spawnenemy`))
  (bind _spawnhealth (`self.spawnhealth`))
  (`|ExecutionSequence`
    (:`then_0`
      (`/Engine/EditorBlueprintResources/StandardMacros.IsValid` _spawnenemy
        (:`Is Valid`
          (`self.K2_DestroyActor` _spawnenemy))))
    (:`then_1`
      (`/Engine/EditorBlueprintResources/StandardMacros.IsValid` _spawnhealth
        (:`Is Valid`
          (`self.K2_DestroyActor` _spawnhealth))))))

(fn `RandomizeWall`
  (`StaticMeshComponent.SetStaticMesh` (`self.WallMesh`) (select `int` (`KismetMathLibrary.RandomIntegerInRange` 0 3) :`0` "/Game/InfiniteMatrix/Meshes/SM_Hole_01.SM_Hole_01" :`1` "/Game/InfiniteMatrix/Meshes/SM_Hole_02.SM_Hole_02" :`2` "/Game/InfiniteMatrix/Meshes/SM_Hole_03.SM_Hole_03" :`3` "/Game/InfiniteMatrix/Meshes/SM_Hole_04.SM_Hole_04" :!type "StaticMesh Object Reference"))
  (`SceneComponent.K2_AddLocalRotation` (`self.WallMesh`) (`KismetMathLibrary.MakeRotator` (`KismetMathLibrary.RandomFloatInRange` 0.0 360.0)) false false))

(fn `UserConstructionScript`
  (`SceneComponent.K2_SetRelativeTransform` (`self.Health`) (`KismetMathLibrary.MakeTransform` (`KismetMathLibrary.MakeVector` (`KismetMathLibrary.RandomFloatInRange` 300.0 2000.0) (`KismetMathLibrary.RandomFloatInRange` -200.0 200.0) (`KismetMathLibrary.RandomFloatInRange` -200.0 200.0))) false false)
  (`SceneComponent.K2_SetRelativeTransform` (`self.Eenemy`) (`KismetMathLibrary.MakeTransform` (`KismetMathLibrary.MakeVector` (`KismetMathLibrary.RandomFloatInRange` 300.0 2000.0) (`KismetMathLibrary.RandomFloatInRange` -200.0 200.0) (`KismetMathLibrary.RandomFloatInRange` -200.0 200.0))) false false))