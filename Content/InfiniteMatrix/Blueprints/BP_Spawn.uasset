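; BP_Spawn is a projectile-like actor that flies forward and destroys enemies for score.
; On BeginPlay it derives its speed from the player's forward speed plus a fixed boost, then Tick teleports it along world X each frame.
; Its Box overlap destroys it on tunnels, enemies or health actors, but only enemies are destroyed with it and award points through the player's AddScore.
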(event `self.ReceiveBeginPlay`
  (bind _asbp_player (cast `/Game/InfiniteMatrix/Blueprints/BP_Player` (`GameplayStatics.GetPlayerPawn` 0)))
  (set `self.As BP Player` _asbp_player)
  (set `self.spawn_speed` (+ (`/Game/InfiniteMatrix/Blueprints/BP_Player.Forward Speed` (`self.As BP Player`)) 1000.0)))

(event `self.ReceiveTick`
  (params (DeltaSeconds :type "Float (single-precision)"))
  (`self.K2_AddActorWorldOffset` (`KismetMathLibrary.MakeVector` (* DeltaSeconds (`self.spawn_speed`))) false true))

(event `self.Box.OnComponentBeginOverlap`
  (params (OverlappedComponent :type "PrimitiveComponent Object Reference") (OtherActor :type "Actor Object Reference") (OtherComp :type "PrimitiveComponent Object Reference") (OtherBodyIndex :type Integer) (bFromSweep :type Boolean) (SweepResult :type "HitResult Structure (by ref)"))
  (cast `/Game/InfiniteMatrix/Blueprints/BP_Tunnel` OtherActor
    (:`then`
      (`self.K2_DestroyActor`))
    (:`CastFailed`
      (bind _asbp_enemy (cast `/Game/InfiniteMatrix/Blueprints/BP_enemy` OtherActor)
        (:`then`
          (`self.K2_DestroyActor` _asbp_enemy)
          (`/Game/InfiniteMatrix/Blueprints/BP_Player.AddScore` (`self.As BP Player`) 5 true)
          (`self.K2_DestroyActor`))
        (:`CastFailed`
          (cast `/Game/InfiniteMatrix/Blueprints/BP_Health` OtherActor)
          (`self.K2_DestroyActor`))))))

(fn `UserConstructionScript`)